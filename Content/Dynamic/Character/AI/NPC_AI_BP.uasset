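; NPC_AI_BP is the AI controller Blueprint for a guard NPC, driving it with the GuardBehavior behavior tree.
; On BeginPlay it initializes the PatrolData blackboard, starts the tree and stores the blackboard component.
; AI perception updates write any sensed actor lacking the "Enemy" tag to the Enemy key, clearing it when sensing of such an actor fails.
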(event `self.ReceiveBeginPlay`
  (bind _blackboardcomponent (`self.UseBlackboard` "/Game/Dynamic/Character/AI/PatrolData.PatrolData"))
  (`self.RunBehaviorTree` "/Game/Dynamic/Character/AI/GuardBehavior.GuardBehavior")
  (set `self.BlackboardComp` _blackboardcomponent))

(event `self.AIPerception.OnTargetPerceptionUpdated`
  (params (Actor :type "Actor Object Reference") (Stimulus :type "AIStimulus Structure"))
  (`self.Update Blackboard Enemy Key` Actor Stimulus))

(fn `Update Blackboard Enemy Key`
  (params (Actor :type "Actor Object Reference") (AIStimulus :type "AIStimulus Structure (by ref)"))
  (bind _blackboardcomp (`self.BlackboardComp`))
  (bind _enemy (`self.Enemy`))
  (`/Engine/EditorBlueprintResources/StandardMacros.IsValid` Actor
    (:`Is Valid`
      (if (`self.ActorHasTag` Actor "Enemy")
        _
        (elif (`.bSuccessfullySensed` (break `AIStimulus` AIStimulus))
          (`BlackboardComponent.SetValueAsObject` _blackboardcomp _enemy Actor)
          (else
            (`BlackboardComponent.ClearValue` _blackboardcomp _enemy)))))))

(fn `UserConstructionScript`)